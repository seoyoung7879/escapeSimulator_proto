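; BP_puzzle is a rotation combination puzzle that controls a linked Door.
; An interact event pitches the given mesh by RotateValue in either direction, then prints its rotation.
; CheckCode maps four meshes to indices and stores whether each pitch matches its Code entry within one degree.
; The all-correct test is disconnected from its loop, so LocalFailed is never set before choosing between opening and closing the door.
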(event EventInteractwithPuzzle
  (params (Component :type Primitive%20Component%20Object%20Reference) (RotateLeft :type Boolean))
  (CallFunction|Rotate Component RotateLeft))

(fn ConstructionScript)

(fn Rotate
  (params (Component :type Primitive%20Component%20Object%20Reference) (Rotate%20left :type Boolean))
  (if Rotate%20left
    (Transformation|AddRelativeRotation Component (Math|Rotator|MakeRotator 0.0 (* (Variables|Default|GetRotateValue) -1.0) 0.0) false false)
    (else
      (Transformation|AddRelativeRotation Component (Math|Rotator|MakeRotator 0.0 (Variables|Default|GetRotateValue) 0.0) false false)))
  (Development|PrintString (Utilities|String|ToString(Rotator) (Variables|/Script/Engine.SceneComponent|GetRelativeRotation Component)))
  (CallFunction|CheckCode Component))

(fn CheckCode
  (params (Component :type Primitive%20Component%20Object%20Reference))
  (bind _door (Variables|Default|GetDoor))
  (if (== Component (Variables|Default|GetStaticMesh1))
    (LocalVariables|SetSelectedMesh 0)
    (Utilities|Array|SetArrayElem (Variables|Default|GetCodeISGood) (LocalVariables|GetSelectedMesh) (Math|Float|NearlyEqual(Float) (Utilities|Array|Get(acopy) (Variables|Default|GetCode) (LocalVariables|GetSelectedMesh)) (.pitch (Variables|/Script/Engine.SceneComponent|GetRelativeRotation Component)) 1.0) :!label _label)
    (bind _array_element (Utilities|Array|ForEachLoopwithBreak (Variables|Default|GetCodeISGood))
      (:Completed
        (if (LocalVariables|GetLocalFailed)
          (Default|CloseDR _door)
          (else
            (Default|OpenDR _door)))))
    (elif (== Component (Variables|Default|GetStaticMesh2))
      (LocalVariables|SetSelectedMesh 1)
      (goto _label)
      (elif (== Component (Variables|Default|GetStaticMesh3))
        (LocalVariables|SetSelectedMesh 2)
        (goto _label)
        (elif (== Component (Variables|Default|GetStaticMesh4))
          (LocalVariables|SetSelectedMesh 3)
          (goto _label))))))