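; Inventory actor component that stores item quantities and data assets in a slot-keyed map, with an input action toggling the UMG inventory widget.
; PickUpItem scans slots to top up matching stacks up to MaxStack, using IsKeyFull, then handles leftovers according to AllowDuplicates and a recorded empty key.
; Add and remove functions edit the map directly, while dropping spawns an A_item only where a box trace ahead of the owner hits.
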(event Input|EnhancedActionEvents|EnhancedInputActionIA_inventory
  (params (ActionValue :type Boolean) (ElapsedSeconds :type Float%20%28double-precision%29) (TriggeredSeconds :type Float%20%28double-precision%29) (InputAction :type Input%20Action%20Object%20Reference :default "/Game/inventory/IA_inventory.IA_inventory"))
  (bind _returnvalue (Game|GetPlayerController 0))
  (bind _returnvalue_2 (Game|GetPlayerController 0))
  (:Started
    (Variables|Default|GetasUMG_inventory
      (:then
        (Variables|/Script/Engine.PlayerController|SetbShowMouseCursor _returnvalue false)
        (Input|SetInputModeGameOnly _returnvalue true)
        (Widget|RemovefromParent (Variables|Default|GetasUMG_inventory))
        (Variables|Default|SetasUMG_inventory 0))
      (:else
        (bind _returnvalue_3 (UserInterface|CreateWidget "/Game/inventory/widget/UMG_inventory.UMG_inventory_C"))
        (bind _output_get (Variables|Default|SetasUMG_inventory _returnvalue_3))
        (UserInterface|Viewport|AddtoViewport _output_get 0)
        (Variables|/Script/Engine.PlayerController|SetbShowMouseCursor _returnvalue_2 false)
        (Input|SetInputModeGameandUI _returnvalue_2 0 "DoNotLock" true false)))))

(event EventBeginPlay
  (Input|AddMappingContext (PlayerController|LocalPlayerSubsystems|GetEnhancedInputLocalPlayerSubsystem (Game|GetPlayerController 0)) "/Game/inventory/IMC_inventory.IMC_inventory" 0 "(bIgnoreAllPressedKeysUntilRelease=True,bForceImmediately=False,bNotifyUserSettings=False)"))

(fn PickUpItem
  (params (item :type A%20Item%20Object%20Reference))
  (bind _structure (Variables|/Game/inventory/item/A_item.A_item_C|Getstructure item))
  (bind _l_index (LocalVariables|GetL-Index))
  (bind _inventory (Variables|Default|Getinventory))
  (bind _l_index_2 (LocalVariables|GetL-Index))
  (bind (_quantity _dataasset) (Utilities|Struct|BreakST_inventory _structure))
  (bind (_returnvalue _remaining) (CallFunction|IsKeyFull _l_index))
  (bind _value (Utilities|Map|Find _inventory _l_index_2))
  (LocalVariables|SetL-quantityIn _quantity)
  (LocalVariables|SetL=dataAssetin _dataasset)
  (while (and (> (LocalVariables|GetL-quantityIn) 0) (< (LocalVariables|GetL-Index) (Variables|Default|GetmaxSize)))
    (Utilities|FlowControl|Sequence
      (:then_0
        (if _returnvalue
          (if (== (.dataasset (.Value (Utilities|Map|Find (Variables|Default|Getinventory) (LocalVariables|GetL-Index)))) (LocalVariables|GetL=dataAssetin))
            (LocalVariables|SetL-foundSameItem true))
          (else
            (bind _output_get (LocalVariables|SetL-remaining _remaining))
            (if (== _output_get -1)
              (if (== -1 (LocalVariables|GetL-emptyKey))
                (LocalVariables|SetL-emptyKey (LocalVariables|GetL-Index)))
              (elif (== (.dataasset _value) (LocalVariables|GetL=dataAssetin))
                (Utilities|Map|Add (Variables|Default|Getinventory) (LocalVariables|GetL-Index) (Utilities|Struct|MakeST_inventory (+ (.quantity _value) (Math|Integer|Clamp(Integer) (LocalVariables|GetL-quantityIn) 0 (LocalVariables|GetL-remaining))) (LocalVariables|GetL=dataAssetin)))
                (LocalVariables|SetL-quantityIn (Math|Integer|Clamp(Integer) (- (LocalVariables|GetL-quantityIn) (LocalVariables|GetL-remaining)) 0 (- (LocalVariables|GetL-quantityIn) (LocalVariables|GetL-remaining))))
                (LocalVariables|SetL-foundSameItem true))))))
      (:then_1
        (Math|Integer|IncrementInt (LocalVariables|GetL-Index)))))
  (if (== (LocalVariables|GetL-quantityIn) 0)
    (return true)
    (elif (and (not (Variables|Default|GetallowDuplicates)) (LocalVariables|GetL-foundSameItem))
      (Default|ModifyQuantity item (LocalVariables|GetL-quantityIn))
      (return false)
      (elif (!= (LocalVariables|GetL-emptyKey) -1)
        (Utilities|Map|Add (Variables|Default|Getinventory) (LocalVariables|GetL-emptyKey) (Utilities|Struct|MakeST_inventory (LocalVariables|GetL-quantityIn) (LocalVariables|GetL=dataAssetin)))
        (return true)
        (else
          (return false))))))

(fn IsKeyFull
  (params (key :type Integer))
  (bind _inventory (Variables|Default|Getinventory))
  (bind (_value _returnvalue) (Utilities|Map|Find _inventory key))
  (bind (_quantity _dataasset) (Utilities|Struct|BreakST_inventory _value))
  (bind _maxstack (Variables|/Game/inventory/item/DA_items.DA_items_C|GetmaxStack _dataasset))
  (bind _returnvalue_2 (- _maxstack _quantity))
  (if _returnvalue
    (return (and (== _returnvalue_2 0) (!= _maxstack 0)) _returnvalue_2)
    (else
      (return true -1))))

(fn ItemAdded
  (params (slotKey :type Integer) (slot%20value :type ST%20Inventory%20Structure))
  (Utilities|Map|Add (Variables|Default|Getinventory) slotKey slot%20value))

(fn ItemDropped
  (params (itemDropped :type ST%20Inventory%20Structure))
  (bind _returnvalue (Components|GetOwner))
  (bind _returnvalue_2 (Transformation|GetActorForwardVector _returnvalue))
  (bind _returnvalue_3 (Transformation|GetActorLocation _returnvalue))
  (bind _returnvalue_4 (* _returnvalue_2 3e+02))
  (bind _returnvalue_5 (+ _returnvalue_3 _returnvalue_4))
  (bind (_outhit _returnvalue_6) (Collision|BoxTraceByChannel _returnvalue_5 (- _returnvalue_5 "") "15.000000,15.000000,15.000000" "0, 0, 0" "TraceTypeQuery1" false (Utilities|Array|MakeArray (Components|GetOwner)) "None"))
  (if _returnvalue_6
    (Game|SpawnActorfromClass "/Game/inventory/item/A_item.A_item_C" (Math|Transform|MakeTransform (.ImpactPoint (Collision|BreakHitResult _outhit)) "0, 0, 0" "1.000000,1.000000,1.000000") "Undefined" "MultiplyWithRoot" 0 itemDropped 0)))

(fn ItemRemoved
  (params (key :type Integer))
  (Utilities|Map|Remove (Variables|Default|Getinventory) key))