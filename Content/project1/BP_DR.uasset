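; BP_DR is an actor Blueprint that rotates a static mesh open and closed, likely a door.
; It stores the mesh's world rotation on BeginPlay as the base orientation.
; OpenDR plays a timeline whose ZAxis track is combined as a yaw offset with that base rotation each update, and CloseDR reverses the same timeline to swing it back.
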(event Custom|CloseDR
  (bind _zaxis (Timeline|DRtimeline Reverse)
    (:Update
      (Transformation|SetWorldRotation (Variables|Debug|GetStaticMeshComponent) (Math|Rotator|CombineRotators (Math|Rotator|MakeRotator 0.0 0.0 _zaxis) (Variables|Default|GetDefaultRotation)) false false))))

(event Custom|OpenDR
  (bind _zaxis (Timeline|DRtimeline Play)
    (:Update
      (Transformation|SetWorldRotation (Variables|Debug|GetStaticMeshComponent) (Math|Rotator|CombineRotators (Math|Rotator|MakeRotator 0.0 0.0 _zaxis) (Variables|Default|GetDefaultRotation)) false false))))

(event EventBeginPlay
  (Variables|Default|SetDefaultRotation (Transformation|GetWorldRotation (Variables|Debug|GetStaticMeshComponent))))

(fn ConstructionScript)